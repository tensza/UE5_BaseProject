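; Player character Blueprint for the demo that detects NPCs with Articy dialogue and lets the player interact with them.
; InteractCheck sphere-traces forward from the actor, accepts BP_NPC hits implementing I_Interact with a valid dialogue ID, and shows or hides the HUD prompt.
; The Move Forward/Backward axis event drives this check continuously, with debug drawing enabled.
; Pressing Interact repeats the check and sends InteractMessage to the returned actor.
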(event EventBeginPlay
  (bind _asdemo_game_mode (Utilities|Casting|CastToDemoGameMode (Game|GetGameMode)))
  (Variables|Default|SetPlayerHUD (Variables|/Game/_Demo/Blueprints/DemoGameMode.DemoGameMode_C|GetPlayerHUD _asdemo_game_mode)))

(event Input|ActionEvents|InputActionInteract
  (params (Key :type Key%20Structure :default "None"))
  (:Pressed
    (bind _actor (CallFunction|InteractCheck))
    (Class|IInteract|Interact(Message) _actor)))

(event Input|AxisEvents|InputAxisMoveForward/Backward
  (params (AxisValue :type Float%20%28single-precision%29))
  (CallFunction|InteractCheck))

(fn ConstructionScript
  (|CallParentFunction))

(fn InteractCheck
  (bind _returnvalue (Transformation|GetActorLocation))
  (bind _playerhud (Variables|Default|GetPlayerHUD))
  (bind _outhit (Collision|SphereTraceByChannel _returnvalue (+ _returnvalue (* (Math|Vector|GetForwardVector (Transformation|GetActorRotation)) 200)) 25.0 "TraceTypeQuery2" false 0 "ForOneFrame"))
  (if (.bblockinghit _outhit)
    (if (Utilities|DoesObjectImplementInterface (.hitactor _outhit) "/Game/_Demo/Blueprints/I_Interact.I_Interact_C")
      (bind _asbp_npc (Utilities|Casting|CastToBP_NPC (.hitactor _outhit)))
      (if (Class|ArticyFunctionLibrary|ArticyIdIsValid (Class|ArticyFunctionLibrary|ArticyRefGetObjectId (Variables|/Game/_Demo/Blueprints/BP_NPC.BP_NPC_C|GetDialogue _asbp_npc)))
        (bind _output_get (LocalVariables|SetInteractActor (.hitactor _outhit)))
        (Default|DisplayMessage _playerhud _output_get true)
        (return (LocalVariables|GetInteractActor))
        (else
          _))))
  (Default|DisplayMessage _playerhud 0 false)
  (return 0))